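; BP_XDGame bridges the game to an external XD platform through typed JSON messages.
; OnXDGameEvent routes messages to handlers that store player info and broadcast game start and hardware axis/button input.
; Req functions send load, progress, motion, renewal and verification requests; many others are empty stubs.
; Verify results pass a timestamp check, then feed SetScript a token-plus-timestamp key and payload for BP_PlayerBase, re-requesting verification on failure.
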(event EventOnXDGameEvent
  (params (Data :type String))
  (bind _bpjson (Class|BpJsonLibrary|ReadJsonfromString Data))
  (bind _out (Class|BpJsonLibrary|GetObjectField _bpjson "data"))
  (Development|PrintString Data)
  (switch string (Class|BpJsonLibrary|GetStringField _bpjson "type")
    (:api_version
      (CallFunction|AskApiVersion (Class|BpJsonLibrary|GetStringField _out "api_version") (Class|BpJsonLibrary|GetStringField _out "app_version")))
    (:player_info
      (CallFunction|OnGetPlayerInfo _out))
    (:game_begin
      (CallFunction|AskGameBegin))
    (:hard_input
      (CallFunction|AskHardInput _out))
    (:renew_result
      (CallFunction|AskRenewResult (Class|BpJsonLibrary|GetNumberField _out "player_no") (Class|BpJsonLibrary|GetStringField _out) (Class|BpJsonLibrary|GetNumberField _out "trade")))
    (:game_over
      (CallFunction|AskGameOver))
    (:verify_result
      (CallFunction|OnSetScript _out))))

(fn AskApiVersion
  (params (ApiVersion :type String) (AppVersion :type String)))

(fn AskHardCharacter)

(fn AskItemInfo)

(fn AskPlayerInfo
  (params (PlayerInfos :type Array%20of%20Struct%20Player%20Information%20Structures))
  (if (> (Utilities|Array|Length PlayerInfos) 0)
    (Default|CallOnAskPlayerInfo)))

(fn AskGameBegin
  (Default|CallOnGameBegin))

(fn AskMotionControlResult)

(fn AskHardInput
  (params (BpJson :type Bp%20Json%20Structure))
  (if (Class|BpJsonLibrary|HasField BpJson "axises")
    (for _array_element (.Out (Class|BpJsonLibrary|GetObjectArrayField BpJson "axises"))
      (switch string (Class|BpJsonLibrary|GetStringField _array_element "axis_no")
        (:0
          (Variables|Default|SetAxisX (Math|Conversions|ToFloat(Integer) (Class|BpJsonLibrary|GetStringField _array_element "value"))))
        (:1
          (Variables|Default|SetAxisY (Math|Conversions|ToFloat(Integer) (Class|BpJsonLibrary|GetStringField _array_element "value"))))
        (:28
          (Variables|Default|SetValue (Math|Conversions|ToFloat(Integer) (Class|BpJsonLibrary|GetStringField _array_element "value")))))))
  (if (Class|BpJsonLibrary|HasField BpJson "buttons")
    (for _array_element_2 (.Out (Class|BpJsonLibrary|GetObjectArrayField BpJson "buttons"))
      (switch string (Class|BpJsonLibrary|GetStringField _array_element_2 "button_no")
        (:4
          (Default|CallOnGetButton4 (Math|Conversions|ToFloat(Integer) (Class|BpJsonLibrary|GetStringField _array_element_2 "value"))))
        (:5
          (Default|CallOnGetButton5 (Math|Conversions|ToFloat(Integer) (Class|BpJsonLibrary|GetStringField _array_element_2 "value"))))
        (:11
          (Default|CallOnGetButton10 (Math|Conversions|ToFloat(Integer) (Class|BpJsonLibrary|GetStringField _array_element_2 "value"))))
        (:12
          (Default|CallOnGetButton11 (Math|Conversions|ToFloat(Integer) (Class|BpJsonLibrary|GetStringField _array_element_2 "value")))))))
  (Default|CallOnGetInput (Variables|Default|GetAxisX) (Variables|Default|GetAxisY) (Variables|Default|Getvalue)))

(fn AskRenewResult
  (params (PlayerNo :type Float%20%28single-precision%29) (PlayerToken :type String) (Trade :type Float%20%28single-precision%29)))

(fn AskBuyItemResult)

(fn AskGameOver)

(fn OnGetPlayerInfo
  (params (BpJson :type Bp%20Json%20Structure))
  (bind (_out _returnvalue) (Class|BpJsonLibrary|GetObjectArrayField BpJson "players"))
  (bind _localplayerinfos (LocalVariables|GetLocalPlayerInfos))
  (if _returnvalue
    (for (_array_element _array_index) _out
      (Utilities|Array|SetArrayElem (LocalVariables|GetLocalPlayerInfos) _array_index (Utilities|Struct|MakeStruct_PlayerInformation (Class|BpJsonLibrary|GetNumberField _array_element "player_no") (Class|BpJsonLibrary|GetStringField _array_element "nick_name") (Class|BpJsonLibrary|GetStringField _array_element "head_url") (Class|BpJsonLibrary|GetStringField _array_element "player_token") (Class|BpJsonLibrary|GetNumberField _array_element "consume") (Class|BpJsonLibrary|GetStringField _array_element "consume_info") (.Out (Class|BpJsonLibrary|GetNumberArrayField _array_element "items"))) true)))
  (Variables|Default|SetPlayerInfos _localplayerinfos)
  (CallFunction|AskPlayerInfo _localplayerinfos))

(fn ReqLoadFinished
  (Class|XDGame|Request (Class|BpJsonLibrary|WriteJsontoString (Class|BpJsonLibrary|SetStringField (Class|BpJsonLibrary|SetStringField (Utilities|Struct|MakeBpJson) "type" "load_finished") "data"))))

(fn ReqPlayProgress
  (params (cur_pos :type Float%20%28single-precision%29) (total_pos :type Float%20%28single-precision%29))
  (Class|XDGame|Request (Class|BpJsonLibrary|WriteJsontoString (Class|BpJsonLibrary|SetObjectField (Class|BpJsonLibrary|SetStringField (Utilities|Struct|MakeBpJson) "type" "play_progress") "data" (Class|BpJsonLibrary|SetStringField (Class|BpJsonLibrary|SetStringField (Utilities|Struct|MakeBpJson) "cur_pos" (Utilities|String|ToString(Float) cur_pos)) "total_pos" (Utilities|String|ToString(Float) total_pos))))))

(fn ReqMotionControl
  (params (DeviceNo :type Float%20%28single-precision%29) (MotionData :type Array%20of%20Struct%20Motion%20Structures))
  (LocalVariables|SetLocalData (Class|BpJsonLibrary|SetStringField (Utilities|Struct|MakeBpJson) "device_no" (Utilities|String|ToString(Float) DeviceNo)))
  (for _array_element MotionData
    (LocalVariables|SetLocalData (Class|BpJsonLibrary|SetStringField (LocalVariables|GetLocalData) (Utilities|String|EnumtoString (.Motion (Utilities|Struct|BreakStruct_Motion _array_element))) (Utilities|String|ToString(Float) (.Value (Utilities|Struct|BreakStruct_Motion _array_element))))))
  (LocalVariables|SetLocalData (Class|BpJsonLibrary|SetObjectField (Class|BpJsonLibrary|SetStringField (Utilities|Struct|MakeBpJson) "type" "motion_control") "data" (LocalVariables|GetLocalData)))
  (Class|XDGame|Request (Class|BpJsonLibrary|WriteJsontoString (LocalVariables|GetLocalData))))

(fn ReqEffectControl
  (params (Effects :type Array%20of%20Struct%20Effect%20Structures) (DeviceNo :type Integer)))

(fn ReqGameScores)

(fn ReqEnterRenew
  (params (PlayerNo :type Float%20%28single-precision%29) (PlayerToken :type String))
  (Class|XDGame|Request (Class|BpJsonLibrary|WriteJsontoString (Class|BpJsonLibrary|SetObjectField (Class|BpJsonLibrary|SetStringField (Utilities|Struct|MakeBpJson) "type" "enter_renew") "data" (Class|BpJsonLibrary|SetStringField (Class|BpJsonLibrary|SetStringField (Utilities|Struct|MakeBpJson) "player_no" (Utilities|String|ToString(Float) PlayerNo)) "player_token" PlayerToken)))))

(fn ReqRenew
  (params (PlayerNo :type Float%20%28single-precision%29) (PlayerToken :type String) (Time :type Float%20%28single-precision%29) (Trade :type Float%20%28single-precision%29)))

(fn ReqBuyItem)

(fn ReqGameEnd
  (params (WaitTime :type Float%20%28single-precision%29)))

(fn ReqGameLottery)

(fn ReqVerify
  (params (PlayerNo :type Float%20%28single-precision%29) (PlayerToken :type String))
  (bind _bpjson (Utilities|Struct|MakeBpJson))
  (bind _bpjson_2 (Utilities|Struct|MakeBpJson))
  (bind _returnvalue (Class|BpJsonLibrary|SetStringField _bpjson "type" "game_verify"))
  (bind _returnvalue_2 (Class|BpJsonLibrary|SetNumberField _bpjson_2 "player_no" PlayerNo))
  (bind _returnvalue_3 (Class|BpJsonLibrary|SetStringField _returnvalue_2 "player_token" PlayerToken))
  (bind _returnvalue_4 (Class|BpJsonLibrary|SetObjectField _returnvalue "data" _returnvalue_3))
  (bind _data (Class|BpJsonLibrary|WriteJsontoString _returnvalue_4))
  (Development|PrintString (Utilities|String|Append "VerifyJson: 
" _data " 
-------------------------------") true true "(R=0.000000,G=0.660000,B=1.000000,A=1.000000)" 5e+01)
  (Class|XDGame|Request _data))

(fn OnSetScript
  (params (BpJson :type Bp%20Json%20Structure))
  (bind _out (Class|BpJsonLibrary|GetStringField BpJson "config_one"))
  (bind _returnvalue (Math|DateTime|Now))
  (bind _out_2 (Class|BpJsonLibrary|GetStringField BpJson "config_two"))
  (bind _playerinfos (Variables|Default|GetPlayerInfos))
  (bind _playerinfos_2 (Variables|Default|GetPlayerInfos))
  (bind _returnvalue_2 (Math|Conversions|ToFloat(Integer) _out))
  (bind _output (Utilities|Array|Get(acopy) _playerinfos_2))
  (bind _output_2 (Utilities|Array|Get(acopy) _playerinfos))
  (bind _player_token (Utilities|Struct|BreakStruct_PlayerInformation _output_2))
  (bind _returnvalue_3 (Utilities|String|Append _player_token _out))
  (if (Utilities|Enum|Equal(Enum) _out "")
    (Development|PrintString "verify_fail" true true "(R=0.000000,G=0.660000,B=1.000000,A=1.000000)" 5e+01 :!label _label)
    (CallFunction|ReqVerify (.player_no _output) (.player_token _output))
    (elif (Utilities|Enum|Equal(Enum) (Class|BpJsonLibrary|GetStringField BpJson "config_two") "")
      (goto _label)
      (else
        (Development|PrintString (Utilities|String|Append "Time: " (Utilities|String|Append (Utilities|String|ToString(Integer) (.year _returnvalue)) "-" (Utilities|String|ToString(Integer) (.month _returnvalue)) "-" (Utilities|String|ToString(Integer) (.day _returnvalue)) "-" (Utilities|String|ToString(Integer) (.hour _returnvalue)) "-" (Utilities|String|ToString(Integer) (.minute _returnvalue)) "-" (Utilities|String|ToString(Integer) (.second _returnvalue)) "-" (Utilities|String|ToString(Integer) (.millisecond _returnvalue))) " | " (Utilities|String|ToString(Float) _returnvalue_2)) true true "(R=0.953191,G=1.000000,B=0.926343,A=1.000000)" 3.6e+03)
        (bind _success (Class|XDGame|CheckTime (Class|KismetMathLibrary|FTrunc64 _returnvalue_2) 86400))
        (if _success
          (if (> (Utilities|Array|Length (Variables|Default|GetPlayerInfos)) 0)
            (Development|PrintString (Utilities|String|Append "config_one: 
" _out " 
config_two: 
" _out_2 " 
key: 
" _returnvalue_3) true true "(R=0.000000,G=0.660000,B=1.000000,A=1.000000)" 5e+01)
            (Class|XDGame|SetScript "Blueprints/Player/BP_PlayerBase_C" (Utilities|Array|MakeArray 95 95 97 95 0) _returnvalue_3 _out_2)
            (Variables|Default|SetKey _returnvalue_3)
            (Variables|Default|SetData _out_2)
            (Default|CallOnSetScripts)
            (else
              (goto _label)))
          (else
            (goto _label)))))))